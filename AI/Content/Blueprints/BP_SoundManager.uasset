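; Sound manager actor that posts Wwise events as pawns enter and leave trigger areas.
; On BeginPlay it binds overlap handlers to every trigger key in the AreaTrigger map, whose values supply each area's enter and leave events.
; Events post on the manager itself, not the trigger.
; Entering turns the trigger's attached TextRender red and caches it; leaving resets only that last cached text to white.
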(event `self.ReceiveBeginPlay`
  (bind _keys (`BlueprintMapLibrary.Map_Keys` (`self.AreaTrigger`)))
  (for _array_element _keys
    (add `self.OnActorBeginOverlap` _array_element (delegate `EV_IM_Start`))
    (add `self.OnActorEndOverlap` _array_element (delegate `EV_IM_End`))))

(event `EV_IM_Start` :!signature `self.OnActorBeginOverlap`
  (params (OverlappedActor :type "Actor Object Reference") (OtherActor :type "Actor Object Reference"))
  (cast `Pawn` OtherActor)
  (bind _astrigger_base (cast `TriggerBase` OverlappedActor))
  (`AkGameplayStatics.PostEvent` (break `/Game/Blueprints/DataType/AkEventPair` (`BlueprintMapLibrary.Map_Find` (`self.AreaTrigger`) _astrigger_base)) self)
  (for _array_element (`self.GetAttachedActors` OverlappedActor)
    (bind _astext_render_actor (cast `TextRenderActor` _array_element))
    (bind _output_get (set `self.CurrentTextRender` _astext_render_actor))
    (`TextRenderComponent.SetTextRenderColor` (`TextRenderActor.TextRender` _output_get) (make `Color` 0 0 255 255))))

(event `EV_IM_End` :!signature `self.OnActorEndOverlap`
  (params (OverlappedActor :type "Actor Object Reference") (OtherActor :type "Actor Object Reference"))
  (cast `Pawn` OtherActor)
  (bind _astrigger_base (cast `TriggerBase` OverlappedActor))
  (`AkGameplayStatics.PostEvent` (`.LeaveEvent_4_1AA587444012179AA21B0EB8C0C9D55A` (break `/Game/Blueprints/DataType/AkEventPair` (`BlueprintMapLibrary.Map_Find` (`self.AreaTrigger`) _astrigger_base))) self)
  (`TextRenderComponent.SetTextRenderColor` (`TextRenderActor.TextRender` (`self.CurrentTextRender`)) (make `Color` 255 255 255 255)))

(fn `UserConstructionScript`)